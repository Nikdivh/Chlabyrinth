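; Resource worker unit for an RTS that shuttles between a resource node and the nearest same-team building.
; SetIsWorking picks the dropoff and starts the trip; Collect halts the unit for a timed gather, then sends it to deliver.
; Dropoff credits the team's player controller and returns it to the node, while SetNotWorking cancels gathering.
; Multicast events drive particles, audio and a selection decal swap showing carried resources.
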(event `MulticastResourceDorppedoff`
  ;[1 1 1] Dropoff reources
  ;;[1 1 1] Multicast resource droppedoff
  (`DecalComponent.SetDecalMaterial` (`self.SelcetionDecal`) "/Game/Materials/SelectedDecal_Mat.SelectedDecal_Mat"))

(event `/Game/Blueprints/ChlabyrinthResourceInterface.Dropoff`
  ;[1 1 1] Dropoff reources
  (if (`self.isWorking?`)
    ;;[1 1 1] If no resource go back to resource node
    (if (`self.hasResource?`)
      ;;[1 1 1] Increment resource amount
      (message `/Game/Blueprints/ChlabyrinthInterface.IncrementResourceAmount` (`GameplayStatics.GetPlayerController` (`self.TeamNumber`)) 10)
      (set `self.hasResource?` false)
      ;;[1 1 1] Multicast resource droppedoff
      (`self.MulticastResourceDorppedoff`)
      ;;[1 1 1] Move to resource node
      (`self.UnitMoveCommand` (`self.K2_GetActorLocation` (`self.ResourceNode`)))
      (else
        (`self.UnitMoveCommand` (`self.K2_GetActorLocation` (`self.ResourceNode`)))))))

(event `MuticastStartCollecting`
  ;[1 1 1] Collect resources
  ;;[1 1 1] Muticast start collecting FX
  (`ActorComponent.SetActive` (`self.ParticleSystem`) true false)
  (`AudioComponent.Play` (`self.Audio`) 0.0))

(event `/Game/Blueprints/ChlabyrinthResourceInterface.Collect`
  ;[1 1 1] Collect resources
  (if (`self.isWorking?`)
    ;;[1 1 1] Already has resource, head to dropoff
    (if (`self.hasResource?`)
      (`self.UnitMoveCommand` (`self.K2_GetActorLocation` (`self.DropoffBuilding`)))
      (else
        ;;[1 1 1] check if collection timer already started
        (if (not (`KismetSystemLibrary.K2_IsValidTimerHandle` (`self.ResourceCollectTimer`)))
          ;;[1 1 1] Stop movement
          (`self.UnitMoveCommand` (`self.K2_GetActorLocation`))
          ;;[1 1 1] Muticast start collecting FX
          (`self.MuticastStartCollecting`)
          ;;[1 1 1] Collect the resource
          (bind _returnvalue (`KismetSystemLibrary.K2_SetTimerDelegate` (delegate `ResourceCollected`) 4.0))
          (set `self.ResourceCollectTimer` _returnvalue))))))

(event `ResourceCollected`
  ;[1 1 1] Collect resources
  ;;[1 1 1] Collect the resource
  (`KismetSystemLibrary.K2_ClearAndInvalidateTimerHandle` (`self.ResourceCollectTimer`))
  (set `self.hasResource?` true)
  ;;[1 1 1] Move to Dropoff
  (`self.UnitMoveCommand` (`self.K2_GetActorLocation` (`self.DropoffBuilding`)))
  ;;[1 1 1] Multicast Done Collecting FX
  (`self.MulticastDoneCollecting`))

(event `MulticastDoneCollecting`
  ;[1 1 1] Collect resources
  ;;[1 1 1] Multicast Done Collecting FX
  (`ActorComponent.SetActive` (`self.ParticleSystem`) false false)
  (`AudioComponent.Stop` (`self.Audio`))
  (`DecalComponent.SetDecalMaterial` (`self.SelcetionDecal`) "/Game/Materials/GoldDecal_Mat.GoldDecal_Mat"))

(event `/Game/Blueprints/ChlabyrinthResourceInterface.SetNotWorking`
  ;[1 1 1] Set not working
  (set `self.isWorking?` false)
  (`KismetSystemLibrary.K2_ClearAndInvalidateTimerHandle` (`self.ResourceCollectTimer`))
  ;;[1 1 1] Multicast not working FX
  (`self.MulticastNotWorking`))

(event `MulticastNotWorking`
  ;[1 1 1] Set not working
  ;;[1 1 1] Multicast not working FX
  (`ActorComponent.SetActive` (`self.ParticleSystem`) false false)
  (`AudioComponent.Stop` (`self.Audio`)))

(event `/Game/Blueprints/ChlabyrinthResourceInterface.SetIsWorking`
  (params (ResourceNode :type "Actor Object Reference"))
  ;[1 1 1] Set is working
  (set `self.isWorking?` true)
  (set `self.ResourceNode` ResourceNode)
  ;;[1 1 1] Find nearest dropoff point
  (bind _outactors (`GameplayStatics.GetAllActorsOfClass` "/Game/Blueprints/Buildings/ParentBuildingClass.ParentBuildingClass_C"))
  (for _array_element _outactors
    (bind _teamnumber (`self.GetTeam` _array_element))
    (if (== _teamnumber (`self.TeamNumber`))
      (bind _returnvalue (`self.GetDistanceTo` _array_element self))
      (if (< _returnvalue (`self.ClosestDropoffBuildingDistance`))
        (set `self.DropoffBuilding` _array_element)
        (set `self.ClosestDropoffBuildingDistance` _returnvalue))))
  ;;[1 1 1] Move to next target
  (if (`self.hasResource?`)
    (`self.UnitMoveCommand` (`self.K2_GetActorLocation` (`self.DropoffBuilding`)))
    (else
      (`self.UnitMoveCommand` (`self.K2_GetActorLocation` (`self.ResourceNode`))))))

(fn `UserConstructionScript`
  (`parent.UserConstructionScript`)
  (`KismetArrayLibrary.Array_Add` (`self.MeshesForTeamColoring`) (`self.Mesh`)))