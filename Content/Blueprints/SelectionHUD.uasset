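; HUD Blueprint for RTS-style box selection of units, holding the SelectedUnits list.
; Press, hold and release events track mouse corners, and DrawHUD draws a translucent blue rectangle between them.
; While drawing, it selects same-team units inside via messages to units and player controller, clears any selected building, and deselects units outside.
; Other events select one unit or clear all; GrabSelectedUnits returns the list.
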(event `/Game/Blueprints/ChlabyrinthInterface.SelectionBoxPressed`
  (bind (_locationx _locationy) (`PlayerController.GetMousePosition` (`GameplayStatics.GetPlayerController` 0)))
  ;[1 1 1] SelectionBoxStart
  (set `self.isDrawing?` true)
  (bind _output_get (set `self.StartMousePosition` (`KismetMathLibrary.MakeVector2D` _locationx _locationy)))
  (set `self.CurrentMousePosition` _output_get))

(event `/Game/Blueprints/ChlabyrinthInterface.SelectionBoxHeld`
  (bind (_locationx _locationy) (`PlayerController.GetMousePosition` (`GameplayStatics.GetPlayerController` 0)))
  ;[1 1 1] SelectionBoxHeld
  (set `self.CurrentMousePosition` (`KismetMathLibrary.MakeVector2D` _locationx _locationy)))

(event `/Game/Blueprints/ChlabyrinthInterface.SelectionBoxReleased`
  ;[1 1 1] SelectionBoxReleased
  (set `self.isDrawing?` false))

(event `self.ReceiveDrawHUD`
  (params (SizeX :type Integer) (SizeY :type Integer))
  (bind (_startmouseposition_x _startmouseposition_y) (`KismetMathLibrary.BreakVector2D` (`self.StartMousePosition`)))
  (bind (_currentmouseposition_x _currentmouseposition_y) (`KismetMathLibrary.BreakVector2D` (`self.CurrentMousePosition`)))
  ;[1 1 1] DRAW RACTANGLE
  (if (`self.isDrawing?`)
    (`self.DrawRect` (struct :`G` 0.201072 :`B` 1.0 :`A` 0.2) _startmouseposition_x _startmouseposition_y (- _currentmouseposition_x _startmouseposition_x) (- _currentmouseposition_y _startmouseposition_y))
    ;[1 1 1] Check for units under the rectangle
    (bind _output_get (set `self.ActorsInRactangle` (`self.GetActorsInSelectionRectangle` "/Game/Blueprints/Units/BP_ParentUnitCalss.BP_ParentUnitCalss_C" (`self.StartMousePosition`) (`self.CurrentMousePosition`) false)))
    (for _array_element _output_get
      ;[1 1 1] Select units
      (bind _teamnumber (message `/Game/Blueprints/ChlabyrinthInterface.GetTeam` _array_element))
      (bind _myteam_ (message `/Game/Blueprints/ChlabyrinthInterface.isOnMyTeam?` (`GameplayStatics.GetPlayerController` 0) _teamnumber))
      (if _myteam_
        (message `/Game/Blueprints/ChlabyrinthInterface.SelectThis` _array_element)
        (`KismetArrayLibrary.Array_AddUnique` (`self.SelectedUnits`) _array_element)
        (message `/Game/Blueprints/ChlabyrinthInterface.ClearSelectedBuilding` (`GameplayStatics.GetPlayerController` 0))))
    ;[1 1 1] Deslect units
    (for _array_element_2 (`self.SelectedUnits`)
      (if (not (`KismetArrayLibrary.Array_Contains` (`self.ActorsInRactangle`) _array_element_2))
        (message `/Game/Blueprints/ChlabyrinthInterface.DeselectThis` _array_element_2)
        (`KismetArrayLibrary.Array_RemoveItem` (`self.SelectedUnits`) _array_element_2)))))

(event `/Game/Blueprints/ChlabyrinthInterface.ClearSelectedUnits`
  (bind _selectedunits (`self.SelectedUnits`))
  ;[1 1 1] Clear Selected Units
  (for _array_element _selectedunits
    (message `/Game/Blueprints/ChlabyrinthInterface.DeselectThis` _array_element))
  (`KismetArrayLibrary.Array_Clear` _selectedunits))

(event `/Game/Blueprints/ChlabyrinthInterface.SelectSingleUnit`
  (params (Unit :type "Actor Object Reference"))
  ;[1 1 1] Select Single Unit
  (message `/Game/Blueprints/ChlabyrinthInterface.SelectThis` Unit)
  (`KismetArrayLibrary.Array_AddUnique` (`self.SelectedUnits`) Unit))

(fn `GetResourceAmount`
  (returns (Amount :type Integer))
  (return 0))

(fn `GetTeam`
  (returns (TeamNumber :type Integer))
  (return 0))

(fn `GrabSelectedUnits`
  (returns (Units :type "Array of Actor Object Reference"))
  (return (`self.SelectedUnits`)))

(fn `isOnMyTeam?`
  (params (TeamNumber :type Integer))
  (returns (`myTeam?` :type Boolean))
  (return false))

(fn `UserConstructionScript`)