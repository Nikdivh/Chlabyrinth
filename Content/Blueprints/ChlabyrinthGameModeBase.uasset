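; Game mode for Chlabyrinth that sets up each joining player with a start camp, camera pawn and team.
; The construction script collects all PlayerStartCamp actors in the level.
; Each new player gets a random camp, possesses a camera pawn spawned at its camera location, and receives the camp, team number and team color through its controller.
; The team number then increments and the used camp leaves the pool, so camps are never shared.
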(event `self.HandleStartingNewPlayer`
  (params (NewPlayer :type "PlayerController Object Reference"))
  ;[1 1 1] Handle starting new player
  ;;[1 1 1] Select random player star camp
  (set `self.SelectedPlayerStartCamp` (`KismetArrayLibrary.Array_Random` (`self.PlayerStartCamps`)))
  ;;[1 1 1] Spawn and posses a new camera pawn for the player
  (bind _returnvalue (`|SpawnActorFromClass` "/Game/Blueprints/CameraPawn.CameraPawn_C" (`SceneComponent.K2_GetComponentToWorld` (`/Game/Blueprints/PlayerStartCamp.CameraLocation` (`self.SelectedPlayerStartCamp`))) "Undefined" "OverrideRootScale" null null))
  (`Controller.Possess` NewPlayer _returnvalue)
  ;;[1 1 1] Send player starting info to player controler
  (message `/Game/Blueprints/ChlabyrinthInterface.SetupPlayerStart` NewPlayer (`self.SelectedPlayerStartCamp`) (`self.TeamNumber`) (`|GetArrayItem` (`self.TeamColors`) (`self.TeamNumber`)))
  ;;[1 1 1] Increment team number and remove player start camp
  (`/Engine/EditorBlueprintResources/StandardMacros.IncrementInt` (`self.TeamNumber`)
    (:`  `
      (`KismetArrayLibrary.Array_RemoveItem` (`self.PlayerStartCamps`) (`self.SelectedPlayerStartCamp`)))))

(fn `UserConstructionScript`
  (bind _outactors (`GameplayStatics.GetAllActorsOfClass` "/Game/Blueprints/PlayerStartCamp.PlayerStartCamp_C"))
  (set `self.PlayerStartCamps` _outactors))