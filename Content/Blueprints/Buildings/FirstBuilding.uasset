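; FirstBuilding is a building Blueprint that offers production actions for a Maria and a resource worker.
; On BeginPlay it creates a widget for each action, adds both to its ActionBoxButtons list and sets each widget's BuildingReference to itself.
; It then calls the parent BeginPlay; the overlap and tick events are disabled, and the construction script only calls the parent.
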(event `self.ReceiveBeginPlay`
  (`|ExecutionSequence`
    (:`then_0`
      (bind _returnvalue (`|CreateWidget` "/Game/Blueprints/Buildings/ProductionWIdgets/ProduceMariaWidget.ProduceMariaWidget_C"))
      (`KismetArrayLibrary.Array_AddUnique` (`self.ActionBoxButtons`) _returnvalue)
      (set `/Game/Blueprints/Buildings/ProductionWIdgets/ProduceMariaWidget.BuildingReference` self _returnvalue))
    (:`then_1`
      (bind _returnvalue_2 (`|CreateWidget` "/Game/Blueprints/Buildings/ProductionWIdgets/ProduceResourceWorkerWidget.ProduceResourceWorkerWidget_C"))
      (`KismetArrayLibrary.Array_AddUnique` (`self.ActionBoxButtons`) _returnvalue_2)
      (set `/Game/Blueprints/Buildings/ProductionWIdgets/ProduceResourceWorkerWidget.BuildingReference` self _returnvalue_2))
    (:`then_2`
      (`parent.ReceiveBeginPlay`))))

(fn `UserConstructionScript`
  (`parent.UserConstructionScript`))