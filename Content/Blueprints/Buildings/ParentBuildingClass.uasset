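; Base class for team-owned RTS buildings that handles selection, team coloring and unit production.
; Selection toggles a decal and a widget filled with action buttons, while dynamic materials tint the mesh and minimap blot.
; A server-only looping timer pulls queued unit classes, tracks progress against each class's default production time, then spawns them with the building's team.
; Overlapping actors receive a server-side drop-off message.
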(event `self.ReceiveActorBeginOverlap`
  (params (OtherActor :type "Actor Object Reference"))
  (`/Engine/EditorBlueprintResources/ActorMacros.Switch Has Authority`
    (:`Authority`
      (message `/Game/Blueprints/ChlabyrinthResourceInterface.Dropoff` OtherActor))))

(event `AddUnitToQueue`
  (params (Unit :type "/Game/Blueprints/Units/ParentUnitCalss Class Reference"))
  (`KismetArrayLibrary.Array_Add` (`self.UnitProductionQueue`) Unit))

(event `/Game/Blueprints/ChlabyrinthInterface.SelectThis`
  (`SceneComponent.SetVisibility` (`self.SelectedDecal`) true false)
  (`UserWidget.AddToViewport` (`self.BuildingSelectedWidget`) 0))

(event `/Game/Blueprints/ChlabyrinthInterface.DeselectThis`
  (`SceneComponent.SetVisibility` (`self.SelectedDecal`) false false)
  (`Widget.RemoveFromParent` (`self.BuildingSelectedWidget`)))

(event `self.ReceiveBeginPlay`
  (`|ExecutionSequence`
    (:`then_0`
      ;[1 1 1] Create Building Selected Widget
      (bind _returnvalue (`|CreateWidget` "/Game/Blueprints/Buildings/BuildingSelectedWidget.BuildingSelectedWidget_C"))
      (set `self.BuildingSelectedWidget` _returnvalue)
      (set `/Game/Blueprints/Buildings/BuildingSelectedWidget.BuildingReference` self _returnvalue)
      (for _array_element (`self.ActionBoxButtons`)
        (`WrapBox.AddChildToWrapBox` (`/Game/Blueprints/Buildings/BuildingSelectedWidget.ActionBox` (`self.BuildingSelectedWidget`)) _array_element)))
    (:`then_1`
      ;[1 1 1] Set Team Color
      (bind _returnvalue_2 (`KismetMaterialLibrary.CreateDynamicMaterialInstance` (`PrimitiveComponent.GetMaterial` (`self.BuildingMesh`) 0)))
      (`MaterialInstanceDynamic.SetVectorParameterValue` _returnvalue_2 "TeamColor" (`self.TeamColor`))
      (`PrimitiveComponent.SetMaterial` (`self.BuildingMesh`) 0 _returnvalue_2)
      (bind _returnvalue_3 (`KismetMaterialLibrary.CreateDynamicMaterialInstance` "/Game/Blueprints/MiniMap/MinimapBlot_Mat.MinimapBlot_Mat"))
      (`MaterialInstanceDynamic.SetVectorParameterValue` _returnvalue_3 "TeamColor" (`self.TeamColor`))
      (`PrimitiveComponent.SetMaterial` (`self.MinimapBlot_Componenet`) 0 _returnvalue_3))
    (:`then_2`
      ;[1 1 1] Unit production
      (`/Engine/EditorBlueprintResources/ActorMacros.Switch Has Authority`
        (:`Authority`
          (`KismetSystemLibrary.K2_SetTimerDelegate` (delegate `ProcessProductionQueue`) (`self.ProductionTimerGranularity`) true))))))

(event `ProcessProductionQueue`
  ;[1 1 1] Unit production
  (if (`self.isProducingUnit?`)
    (bind _output_get (set `self.ProductionTImeSpent` (+ (`self.ProductionTImeSpent`) (`self.ProductionTimerGranularity`))))
    (bind _output_get_2 (set `self.ProductionProgress` (/ _output_get (`self.ProductionTimeNeeded`))))
    (if (>= _output_get_2 1.0)
      (`|SpawnActorFromClass` (`self.UnitBeingProduced`) (`KismetMathLibrary.MakeTransform` (`SceneComponent.K2_GetComponentLocation` (`self.UnitSpawnPoint`))) "AdjustIfPossibleButAlwaysSpawn" "OverrideRootScale" null (`self.TeamNumber`) (`self.TeamColor`) null)
      (set `self.ProductionProgress` 0.0)
      (set `self.ProductionTImeSpent` 0.0)
      (set `self.UnitBeingProduced` null)
      (set `self.isProducingUnit?` false))
    (elif (> (`KismetArrayLibrary.Array_Length` (`self.UnitProductionQueue`)) 0)
      (bind _output_get_3 (set `self.UnitBeingProduced` (`|GetArrayItem` (`self.UnitProductionQueue`))))
      (set `self.ProductionTimeNeeded` (`.ProductionTime` (defaults `Object` _output_get_3)))
      (`KismetArrayLibrary.Array_Remove` (`self.UnitProductionQueue`))
      (set `self.isProducingUnit?` true))))

(fn `GetResourceAmount`
  (returns (Amount :type Integer))
  (return 0))

(fn `GetTeam`
  (returns (TeamNumber :type Integer))
  (return (`self.TeamNumber`)))

(fn `GrabSelectedUnits`
  (returns (Units :type "Array of Actor Object Reference"))
  (return))

(fn `isOnMyTeam?`
  (params (TeamNumber :type Integer))
  (returns (`myTeam?` :type Boolean))
  (return false))

(fn `UserConstructionScript`)