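; RTS player controller that handles mouse selection, unit orders, team identity and resource amount.
; Left clicks select friendly buildings and drive the HUD's selection box, while right clicks send HUD-selected units to move or work resource nodes, with cursor feedback.
; Unit orders and building production queues go through server passthrough events.
; On authority it spawns each starting camp's building and three workers; the local controller creates the main UI with a camera-aligned minimap.
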(event `self.IncrementResourceAmount`
  (params (Amount :type Integer))
  ;[1 1 1] Increment Resource Amount
  (set `self.ResourceAmount` (+ Amount (`self.ResourceAmount`))))

(event `self.ProduceUnit`
  (params (Building :type "/Game/Blueprints/Buildings/ParentBuildingClass Object Reference") (Unit :type "/Game/Blueprints/Units/BP_ParentUnitCalss Class Reference"))
  ;[0.9531 1 0.9062] Produce Unit
  (`self.ServerAddUnitToQueue` Building Unit))

(event `ServerAddUnitToQueue`
  (params (Building :type "/Game/Blueprints/Buildings/ParentBuildingClass Object Reference") (Unit :type "/Game/Blueprints/Units/BP_ParentUnitCalss Class Reference"))
  ;[0.9531 1 0.9062] Produce Unit
  (`/Game/Blueprints/Buildings/ParentBuildingClass.AddUnitToQueue` Building Unit))

(event `self.SetupPlayerStart`
  (params (PlayerStartCamp :type "/Game/Blueprints/PlayerStartCamp Object Reference") (TeamNumber :type Integer) (TeamColor :type "LinearColor Structure"))
  ;[1 1 1] Setup player start
  (`/Engine/EditorBlueprintResources/ActorMacros.Switch Has Authority`
    (:`Authority`
      (set `self.Team Number` TeamNumber)
      (set `self.Team Color` TeamColor)
      (`self.SpawnPlayerStartingCamp` PlayerStartCamp))))

(event `self.ClearSelectedBuilding`
  (bind _selectedbuilding (`self.SelectedBuilding`))
  ;[1 1 1] Clear selected Buildings
  (`/Engine/EditorBlueprintResources/StandardMacros.IsValid` _selectedbuilding
    (:`Is Valid`
      (message `/Game/Blueprints/ChlabyrinthInterface.DeselectThis` _selectedbuilding)
      (set `self.SelectedBuilding` null))))

(event `self.AddUnitToSelectedUnitsArea`
  (params (SelectedUnitWidget :type "UserWidget Object Reference"))
  ;[1 1 1] Add unit to selection area
  (`HorizontalBox.AddChildToHorizontalBox` (`/Game/MainUI_Widget.UnitsBox` (`self.MainUI_Widget`)) SelectedUnitWidget))

(event `self.ReceiveBeginPlay`
  ;[1 1 1] Begin play
  (if (`self.IsLocalPlayerController`)
    (`|ExecutionSequence`
      (:`then_0`
        (`self.SetupGameMode_and_Mouse`))
      (:`then_1`
        (`self.CreateMainUI_Widget`)))))

(event `self.ReceiveTick`
  (params (DeltaSeconds :type "Float (single-precision)"))
  ;[1 1 1] Left Mouse Click
  (if (`self.isLefMouseButtonPressed?`)
    (message `/Game/Blueprints/ChlabyrinthInterface.SelectionBoxHeld` (`self.GetHUD`))))

(event `Key|LeftMouseButton`
  (params (Key :type "Key Structure"))
  (bind _returnvalue (`self.GetHUD`))
  ;[1 1 1] Left Mouse Click
  (:`Pressed`
    (set `self.isLefMouseButtonPressed?` true)
    (`self.HandleBuildingClick`)
    (message `/Game/Blueprints/ChlabyrinthInterface.SelectionBoxPressed` _returnvalue))
  (:`Released`
    (set `self.isLefMouseButtonPressed?` false)
    (message `/Game/Blueprints/ChlabyrinthInterface.SelectionBoxReleased` _returnvalue)))

(event `Key|RightMouseButton`
  (params (Key :type "Key Structure"))
  (bind (_location _hitactor) (`self.RightClickHitResultUnderCursor`))
  ;[1 1 1] Right mouse click
  (:`Pressed`
    (if (== (`GameplayStatics.GetObjectClass` _hitactor) "/Game/Blueprints/ResourceNode.ResourceNode_C")
      (`self.HandleRightClickResourceNode` _hitactor)
      (else
        (`self.HandleRightClickToMoveUnits` _location)))))

(event `ServerPassthroughSetIsWorking`
  (params (Unit :type "Actor Object Reference") (ResourceNode :type "Actor Object Reference"))
  ;[0 1 0.1062] Right click server passthrough functions
  (message `/Game/Blueprints/ChlabyrinthResourceInterface.SetIsWorking` Unit ResourceNode))

(event `ServerPassthroughSetNotWorking`
  (params (Unit :type "Actor Object Reference"))
  ;[0 1 0.1062] Right click server passthrough functions
  (message `/Game/Blueprints/ChlabyrinthResourceInterface.SetNotWorking` Unit))

(event `ServerPassthroughUnitMoveCommand`
  (params (Unit :type "Actor Object Reference") (Location :type "Vector Structure"))
  ;[0 1 0.1062] Right click server passthrough functions
  (message `/Game/Blueprints/ChlabyrinthInterface.UnitMoveCommand` Unit Location))

(fn `GetResourceAmount`
  (returns (Amount :type Integer))
  (return (`self.ResourceAmount`)))

(fn `GetTeam`
  (returns (TeamNumber :type Integer))
  (return 0))

(fn `GrabSelectedUnits`
  (returns (Units :type "Array of Actor Object Reference"))
  (return))

(fn `isOnMyTeam?`
  (params (TeamNumber :type Integer))
  (returns (`myTeam?` :type Boolean))
  (return (== TeamNumber (`self.Team Number`))))

(fn `UserConstructionScript`)